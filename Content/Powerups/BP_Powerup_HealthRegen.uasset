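; Health regeneration powerup that heals the player over time while it runs.
; On each powerup tick it looks up the SHealthComponent on player 0's pawn, regardless of who triggered it, and heals by HealingAmount.
; Activation state changes toggle the mesh and its children, hiding them while active, and expiry destroys the actor.
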(event `self.OnPowerupStateChanged`
  (params (bNewIsActive :type Boolean))
  (`SceneComponent.SetVisibility` (`self.StaticMesh`) (not bNewIsActive) true))

(event `self.OnExpired`
  (`self.K2_DestroyActor`))

(event `self.OnPowerupTicked`
  (bind _returnvalue (`self.GetComponentByClass` (`GameplayStatics.GetPlayerPawn` 0) "/Script/CoopGame.SHealthComponent"))
  (`/Engine/EditorBlueprintResources/StandardMacros.IsValid` _returnvalue
    (:`Is Valid`
      (`SHealthComponent.Heal` _returnvalue (`self.HealingAmount`)))))

(fn `UserConstructionScript`)